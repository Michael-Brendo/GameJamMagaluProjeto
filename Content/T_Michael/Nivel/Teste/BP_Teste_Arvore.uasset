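; Test tree actor that acts as a wood (Madeira) resource for the player to gather.
; A Sphere overlap toggles PodeColetarMadeira on the ThirdPersonCharacter as it enters and leaves.
; The Interagir event waits through a short Delay, then adds one wood to player 0's character, clamped to a small maximum.
; Interagir does not check the range flag itself, and the tree is never depleted.
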(event `/Game/T_Michael/Nivel/Teste/BP_Interativo.Interagir`
  ;[1 1 1] Coleta Madeira
  (`KismetSystemLibrary.Delay` 1.0)
  (bind _asthird_person_character (cast `/Game/ThirdPersonBP/Blueprints/ThirdPersonCharacter` (`GameplayStatics.GetPlayerCharacter` 0)))
  (set `/Game/ThirdPersonBP/Blueprints/ThirdPersonCharacter.Madeira` (`KismetMathLibrary.Clamp` (+ (`/Game/ThirdPersonBP/Blueprints/ThirdPersonCharacter.Madeira` _asthird_person_character) 1) 0 10) _asthird_person_character))

(event `self.Sphere.OnComponentBeginOverlap`
  (params (OverlappedComponent :type "PrimitiveComponent Object Reference") (OtherActor :type "Actor Object Reference") (OtherComp :type "PrimitiveComponent Object Reference") (OtherBodyIndex :type Integer) (bFromSweep :type Boolean) (SweepResult :type "HitResult Structure (by ref)"))
  (bind _asthird_person_character (cast `/Game/ThirdPersonBP/Blueprints/ThirdPersonCharacter` OtherActor))
  (set `/Game/ThirdPersonBP/Blueprints/ThirdPersonCharacter.PodeColetarMadeira` true _asthird_person_character))

(event `self.Sphere.OnComponentEndOverlap`
  (params (OverlappedComponent :type "PrimitiveComponent Object Reference") (OtherActor :type "Actor Object Reference") (OtherComp :type "PrimitiveComponent Object Reference") (OtherBodyIndex :type Integer))
  (bind _asthird_person_character (cast `/Game/ThirdPersonBP/Blueprints/ThirdPersonCharacter` OtherActor))
  (set `/Game/ThirdPersonBP/Blueprints/ThirdPersonCharacter.PodeColetarMadeira` false _asthird_person_character))

(fn `UserConstructionScript`)